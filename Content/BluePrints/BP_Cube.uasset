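; BP_Cube is a player-controlled cube that rolls by applying physics torque to its static mesh.
; The Forward and Left/Right input axes add scaled angular acceleration around the Y and X axes, ignoring mass.
; Tick prints the mesh's world rotation as debug output, and a rotation reset node is left unconnected.
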(event `InputAxis|Forward`
  (params (AxisValue :type "Float (single-precision)"))
  (`PrimitiveComponent.AddTorqueInRadians` (`self.StaticMesh`) (`KismetMathLibrary.MakeVector` 0.0 (* AxisValue 12.0)) "None" true))

(event `self.ReceiveTick`
  (params (DeltaSeconds :type "Float (single-precision)"))
  (`KismetSystemLibrary.PrintString` (`KismetStringLibrary.Conv_RotatorToString` (`SceneComponent.K2_GetComponentRotation` (`self.StaticMesh`)))))

(event `InputAxis|Left/Right`
  (params (AxisValue :type "Float (single-precision)"))
  (`PrimitiveComponent.AddTorqueInRadians` (`self.StaticMesh`) (`KismetMathLibrary.MakeVector` (* AxisValue 12.0)) "None" true))

(fn `UserConstructionScript`)